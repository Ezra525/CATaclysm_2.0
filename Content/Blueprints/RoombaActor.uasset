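; Roomba pawn that roams around its spawn point and detects the player, handing state to its AI controller's behavior through the blackboard.
; On BeginPlay it stores its starting location and writes that and its RoamingRange to the blackboard.
; PawnSensing reports seen pawns; the first time it sees player character 0, it caches it and sets the PlayerPawn key, which is never cleared here.
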(event OnSeePawn(PawnSensing)
  (params (Pawn :type Pawn%20Object%20Reference))
  (if (== Pawn (Game|GetPlayerCharacter 0))
    (Utilities|IsValid (Variables|Default|GetPlayerPawn)
      (:Is%20Not%20Valid
        (bind _output_get (Variables|Default|SetPlayerPawn Pawn))
        (AI|Components|Blackboard|SetValueasObject (AI|GetBlackboard (AI|GetAIController self)) (Utilities|Name|MakeLiteralName "PlayerPawn") _output_get)))))

(event EventBeginPlay
  (bind _self self)
  (bind _returnvalue (AI|GetAIController _self))
  (bind _returnvalue_2 (AI|GetBlackboard _returnvalue))
  (Variables|Default|SetStartingLocation (Transformation|GetActorLocation))
  (AI|Components|Blackboard|SetValueasFloat _returnvalue_2 (Utilities|Name|MakeLiteralName "RoamingRange") (Variables|Default|GetRoamingRange))
  (AI|Components|Blackboard|SetValueasVector _returnvalue_2 (Utilities|Name|MakeLiteralName "StartingLocation") (Variables|Default|GetStartingLocation)))

(event Collision|EventActorBeginOverlap
  (params (OtherActor :type Actor%20Object%20Reference)))

(event EventTick
  (params (DeltaSeconds :type Float%20%28single-precision%29)))

(fn ConstructionScript)