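; Roomba enemy pawn that detects the player and opens a game-over level when it hits them.
; On start it seeds its AI blackboard with roaming range and starting location.
; Pawn sensing latches the player into the blackboard, after which Tick rotates the pawn to face them.
; Heard noises are stored locally, while a separate HandleSoundSense function, uncalled here, writes hearing-stimulus locations to the blackboard as TargetLocation.
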(event OnSeePawn(PawnSensing)
  (params (Pawn :type Pawn%20Object%20Reference))
  (if (== Pawn (Game|GetPlayerCharacter 0))
    (Utilities|IsValid (Variables|Default|GetPlayerPawn)
      (:Is%20Not%20Valid
        (bind _output_get (Variables|Default|SetPlayerPawn Pawn))
        (AI|Components|Blackboard|SetValueasObject (AI|GetBlackboard (AI|GetAIController self)) (Utilities|Name|MakeLiteralName "PlayerPawn") _output_get)))))

(event OnHearNoise(PawnSensing)
  (params (Instigator :type Pawn%20Object%20Reference) (Location :type Vector%20%28by%20ref%29 :default "0, 0, 0") (Volume :type Float%20%28single-precision%29))
  (Variables|Default|SetHearedNoise Location))

(event EventBeginPlay
  (bind _self self)
  (bind _returnvalue (AI|GetAIController _self))
  (bind _returnvalue_2 (AI|GetBlackboard _returnvalue))
  (Variables|Default|SetStartingLoaction (Transformation|GetActorLocation))
  (AI|Components|Blackboard|SetValueasFloat _returnvalue_2 (Utilities|Name|MakeLiteralName "RoamingRange") (Variables|Default|GetRoamingRange))
  (AI|Components|Blackboard|SetValueasVector _returnvalue_2 (Utilities|Name|MakeLiteralName "StartingLocation") (Variables|Default|GetStartingLoaction)))

(event Collision|EventActorBeginOverlap
  (params (OtherActor :type Actor%20Object%20Reference)))

(event EventTick
  (params (DeltaSeconds :type Float%20%28single-precision%29))
  (bind _returnvalue (Transformation|GetActorLocation))
  (bind _playerpawn (Variables|Default|GetPlayerPawn))
  (bind _returnvalue_2 (Transformation|GetActorLocation _playerpawn))
  (bind _returnvalue_3 (Math|Rotator|FindLookatRotation _returnvalue _returnvalue_2))
  (if (== _playerpawn (Game|GetPlayerCharacter 0))
    (Transformation|SetActorRotation (Math|Rotator|MakeRotator (.roll _returnvalue_3) 0.0 (.yaw _returnvalue_3)))))

(event Collision|EventHit
  (params (MyComp :type Primitive%20Component%20Object%20Reference) (Other :type Actor%20Object%20Reference) (OtherComp :type Primitive%20Component%20Object%20Reference) (bSelfMoved :type Boolean) (HitLocation :type Vector :default "0, 0, 0") (HitNormal :type Vector :default "0, 0, 0") (NormalImpulse :type Vector :default "0, 0, 0") (Hit :type Hit%20Result%20Structure%20%28by%20ref%29))
  (if (== Other (Game|GetPlayerCharacter 0))
    (Game|OpenLevel(byObjectReference) "/Game/Maps/GameOverLevel.GameOverLevel")))

(fn ConstructionScript)

(fn HandleSoundSense
  (params (Stimulus :type AI%20Stimulus%20Structure%20%28by%20ref%29))
  (bind _returnvalue (Class|AIPerceptionSystem|GetSenseClassforStimulus Stimulus))
  (if (== _returnvalue "/Script/AIModule.AISense_Hearing")
    (AI|Components|Blackboard|SetValueasVector (AI|GetBlackboard (AI|GetAIController self)) (Utilities|Name|MakeLiteralName "TargetLocation") (.StimulusLocation (Utilities|Struct|BreakAIStimulus Stimulus)))))